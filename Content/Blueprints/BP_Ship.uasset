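; BP_Ship is a boardable ship Blueprint that the player occupies by interacting with it.
; On BeginPlay it caches the player's BP_FirstPersonCharacter.
; Interact works only while the ship is unoccupied: it sets the occupied flag, assigns itself as the character's CurrentShip and calls OnShipOccupied on the character.
; It contains no movement or exit logic.
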(event EventBeginPlay
  (bind _asbp_first_person_character (Utilities|Casting|CastToBP_FirstPersonCharacter (Game|GetPlayerCharacter 0)))
  (Variables|Default|SetPlayer _asbp_first_person_character))

(event EventInteract
  (bind _player (Variables|Default|GetPlayer))
  (if (not (Variables|Default|GetOnShipOccupied))
    (Variables|Default|SetOnShipOccupied true)
    (Variables|/Game/FirstPerson/Blueprints/BP_FirstPersonCharacter.BP_FirstPersonCharacter_C|SetCurrentShip _player self)
    (Default|OnShipOccupied _player)))

(fn ConstructionScript)